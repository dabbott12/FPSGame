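; Enemy pawn that chases the player and enters a timed attack state when within reach.
; BeginPlay caches the player character, then Tick reissues AI MoveTo toward it and snaps yaw to face it while the enemy is neither Dead nor Attacking.
; A successful move sets Attacking for a fixed delay, pausing the chase; this graph applies no damage and never sets Dead.
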(event `self.ReceiveBeginPlay`
  ;[1 1 1] Creating Player Object
  (bind _asplayer (cast `/Game/Blueprints/Player` (`GameplayStatics.GetPlayerCharacter` 0)))
  (set `self.Player` _asplayer))

(event `self.ReceiveTick`
  (params (DeltaSeconds :type "Float (single-precision)"))
  ;[1 1 1] If Enemy is NOT Dead or Attacking, Move Towards Player
  (if (not (or (`self.Dead`) (`self.Attacking`)))
    (`|AIMoveTo` self (0.0 0.0 0.0) (`self.Player`) (`self.AttackStartDistance`)
      (:`then`
        ;[1 1 1] Rotate Towards Player
        (`self.K2_SetActorRotation` (`KismetMathLibrary.MakeRotator` 0.0 0.0 (.yaw (`KismetMathLibrary.FindLookAtRotation` (`self.K2_GetActorLocation`) (`self.K2_GetActorLocation` (`self.Player`)))))))
      (:`OnSuccess`
        ;[1 1 1] Attacking
        (if (not (`self.Attacking`))
          (set `self.Attacking` true)
          (`KismetSystemLibrary.Delay` 2.6)
          (set `self.Attacking` false))))))

(fn `UserConstructionScript`)