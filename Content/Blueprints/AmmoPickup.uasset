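; Ammo pickup actor that gives ammo to the Player who walks into it.
; Tick spins the static mesh around yaw at RotateSpeed, scaled by delta time.
; On overlap with a Player, it adds AmmoToAdd through AddAmmo and destroys itself, unless the player's ammo is already at max, when it only prints a message.
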(event `self.ReceiveTick`
  (params (DeltaSeconds :type "Float (single-precision)"))
  ;[1 1 1] Spin The Ammo Pickup
  (`SceneComponent.K2_AddWorldRotation` (`self.StaticMesh`) (`KismetMathLibrary.MakeRotator` 0.0 0.0 (* DeltaSeconds (`self.RotateSpeed`))) false false))

(event `self.ReceiveActorBeginOverlap`
  (params (OtherActor :type "Actor Object Reference"))
  ;[1 1 1] Player Picks Up Ammo Pickup
  (bind _asplayer (cast `/Game/Blueprints/Player` OtherActor))
  (if (== (`/Game/Blueprints/Player.MaxAmmo` _asplayer) (`/Game/Blueprints/Player.CurrentAmmo` _asplayer))
    (`KismetSystemLibrary.PrintString` "Already have max ammo!")
    (else
      (`/Game/Blueprints/Player.AddAmmo` _asplayer (`self.AmmoToAdd`))
      (`self.K2_DestroyActor`))))

(fn `UserConstructionScript`)