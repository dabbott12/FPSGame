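; A health pickup actor that restores health to the player on contact.
; Its mesh spins around the yaw axis every tick at a configurable rotate speed.
; On overlap it casts to Player, adds the configured health and destroys itself, unless the player is already at max health, in which case it only prints a message.
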(event `self.ReceiveTick`
  (params (DeltaSeconds :type "Float (single-precision)"))
  ;[1 1 1] Spin The Health Pickup
  (`SceneComponent.K2_AddWorldRotation` (`self.StaticMesh`) (`KismetMathLibrary.MakeRotator` 0.0 0.0 (* DeltaSeconds (`self.RotateSpeed`))) false false))

(event `self.ReceiveActorBeginOverlap`
  (params (OtherActor :type "Actor Object Reference"))
  ;[1 1 1] Player Picks Up Health Pickup
  (bind _asplayer (cast `/Game/Blueprints/Player` OtherActor))
  (if (== (`/Game/Blueprints/Player.MaxHealth` _asplayer) (`/Game/Blueprints/Player.CurrentHealth` _asplayer))
    (`KismetSystemLibrary.PrintString` "Already have max health!")
    (else
      (`/Game/Blueprints/Player.AddHealth` _asplayer (`self.HealthToAdd`))
      (`self.K2_DestroyActor`))))

(fn `UserConstructionScript`)